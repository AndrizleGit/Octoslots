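; Octopus player character Blueprint that provides auto-aimed shooting and footstep audio.
; AutoShoot finds the nearest actor tagged Enemy and spawns a PlayerProjectile rotated toward it, falling back to the character's own rotation when none is found.
; PlayFootstepSfx steps through an array of sounds in looping order, playing each in 2D with slight random pitch variation.
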(fn `AutoShoot`
  (bind _returnvalue (`self.K2_GetActorLocation`))
  (bind _outactors (`GameplayStatics.GetAllActorsWithTag` "Enemy"))
  (bind (_distance _returnvalue_2) (`GameplayStatics.FindNearestActor` _returnvalue _outactors))
  (`/Engine/EditorBlueprintResources/StandardMacros.IsValid` _returnvalue_2
    (:`Is Valid`
      (`|SpawnActorFromClass` "/Script/OctoPirate.PlayerProjectile" (`KismetMathLibrary.MakeTransform` _returnvalue (`KismetMathLibrary.FindLookAtRotation` _returnvalue (`self.K2_GetActorLocation` _returnvalue_2))) "Undefined" "MultiplyWithRoot" null null))
    (:`Is Not Valid`
      (`|SpawnActorFromClass` "/Script/OctoPirate.PlayerProjectile" (`KismetMathLibrary.MakeTransform` _returnvalue (`self.K2_GetActorRotation`)) "Undefined" "MultiplyWithRoot" null null))))

(fn `Play Footstep Sfx`
  (bind _sound_index (`self.Sound Index`))
  (`GameplayStatics.PlaySound2D` (`|GetArrayItem` (`self.Footstep Sfx`) (`self.Sound Index`)) 1.0 (`KismetMathLibrary.RandomFloatInRange` 0.9 1.1) 0.0 null null)
  (`/Engine/EditorBlueprintResources/StandardMacros.IncrementInt` _sound_index
    (:`  `
      (if (>= _sound_index (`KismetArrayLibrary.Array_Length` (`self.Footstep Sfx`)))
        (set `self.Sound Index` 0)))))

(fn `UserConstructionScript`)