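; BP_OctopirateGameInstance is the Octopirate game instance that owns the save object holding meta progress.
; On Init it loads the BP_OctoSlotsSaveGame from a single fixed slot, or creates a new one in memory if none exists.
; GetMetaProgress returns that object's SaveGame data, and SaveMetaProgress writes the object back to the slot, either synchronously or asynchronously.
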(event `self.ReceiveInit`
  (bind _saveslot1 (`self.SaveSlot1`))
  (bind _returnvalue (`GameplayStatics.DoesSaveGameExist` _saveslot1))
  (if _returnvalue
    (bind _returnvalue_2 (`GameplayStatics.LoadGameFromSlot` _saveslot1))
    (bind _asbp_octo_slots_save_game (cast `/Game/Blueprints/BP_OctoSlotsSaveGame` _returnvalue_2))
    (set `self.CurrentSaveObject` _asbp_octo_slots_save_game)
    (else
      (bind _returnvalue_3 (`GameplayStatics.CreateSaveGameObject` "/Game/Blueprints/BP_OctoSlotsSaveGame.BP_OctoSlotsSaveGame_C"))
      (set `self.CurrentSaveObject` _returnvalue_3))))

(event `/Game/Blueprints/BPI_SaveSystem.SaveMetaProgress`
  (params (bIsAsync :type Boolean) (DataToSave :type "/Game/Blueprints/UI/S_MetaProgression Structure"))
  (bind _saveslot1 (`self.SaveSlot1`))
  (bind _currentsaveobject (`self.CurrentSaveObject`))
  (if bIsAsync
    (`AsyncActionHandleSaveGame.AsyncSaveGameToSlot` _currentsaveobject _saveslot1)
    (else
      (`GameplayStatics.SaveGameToSlot` _currentsaveobject _saveslot1))))

(fn `GetMetaProgress`
  (returns (SavedData :type "/Game/Blueprints/UI/S_MetaProgression Structure"))
  (return (`/Game/Blueprints/BP_OctoSlotsSaveGame.SaveGame` (`self.CurrentSaveObject`))))