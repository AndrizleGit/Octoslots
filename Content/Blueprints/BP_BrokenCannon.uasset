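; BP_BrokenCannon is a cannon that the octopus player repairs by bringing it fragments.
; When an octopus character overlaps its box while unassembled, it takes fragments from that character's TreasureMap via SubmitCannonFragment and adds them to a running count.
; Reaching the maximum count calls ShootCannon, which currently only marks the cannon as assembled so further overlaps are ignored.
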(event `Shoot Cannon`
  (set `self.bAssambled` true))

(event `self.Box.OnComponentBeginOverlap`
  (params (OverlappedComponent :type "PrimitiveComponent Object Reference") (OtherActor :type "Actor Object Reference") (OtherComp :type "PrimitiveComponent Object Reference") (OtherBodyIndex :type Integer) (bFromSweep :type Boolean) (SweepResult :type "HitResult Structure (by ref)"))
  (if (not (`self.bAssambled`))
    (bind _asbp_octopus_character (cast `/Game/Blueprints/BP_OctopusCharacter` OtherActor))
    (bind _returnvalue (`TreasureMapComponent.SubmitCannonFragment` (`/Game/Blueprints/BP_OctopusCharacter.TreasureMap` _asbp_octopus_character)))
    (bind _output_get (set `self.CurrentFragment` (+ (`self.CurrentFragment`) _returnvalue)))
    (if (>= _output_get (`self.MaxFragment`))
      (`self.Shoot Cannon`))))

(fn `UserConstructionScript`)