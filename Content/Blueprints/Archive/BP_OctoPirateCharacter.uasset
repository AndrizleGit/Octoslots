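; Octopus pirate character, archived, with timed auto-attack, movement and attack-speed bonuses, cycling footstep sounds, and mesh physics on any damage.
; A looping timer calls AutoShoot, but that function is empty; its nearest-"Enemy" aim-and-spawn logic is disconnected.
; The attack-speed multiplier scales the timer interval and restarts it.
; Removing the multiplier starts a new timer without clearing the running one.
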(event `self.ReceiveAnyDamage`
  (params (Damage :type "Float (single-precision)") (DamageType :type "DamageType Object Reference") (InstigatedBy :type "Controller Object Reference") (DamageCauser :type "Actor Object Reference"))
  (`PrimitiveComponent.SetSimulatePhysics` (`self.Mesh`) true))

(event `self.ReceiveBeginPlay`
  (set `self.CurrentAttackSpeed` (`self.DefaultAttackSpeed`))
  (set `CharacterMovementComponent.MaxWalkSpeed` (`self.DefaultWalkSpeed`) (`self.CharacterMovement`))
  (bind _returnvalue (`KismetSystemLibrary.K2_SetTimerDelegate` (delegate `Shoot`) (`self.CurrentAttackSpeed`) true true))
  (set `self.AttackTimerHandle` _returnvalue))

(event `Shoot`
  (`self.AutoShoot`))

(event `self.AddMovementSpeedBonus`
  (params (Bonus :type "Float (single-precision)"))
  (set `CharacterMovementComponent.MaxWalkSpeed` (+ Bonus (`self.DefaultWalkSpeed`)) (`self.CharacterMovement`)))

(event `self.RemoveMovementSpeedBonus`
  (set `CharacterMovementComponent.MaxWalkSpeed` (`self.DefaultWalkSpeed`) (`self.CharacterMovement`)))

(event `self.ApplyAttackSpeedMultiplier`
  (params (Multiplier :type "Float (single-precision)"))
  (`KismetSystemLibrary.K2_ClearAndInvalidateTimerHandle` (`self.AttackTimerHandle`))
  (bind _output_get (set `self.CurrentAttackSpeed` (* Multiplier (`self.DefaultAttackSpeed`))))
  (bind _returnvalue (`KismetSystemLibrary.K2_SetTimerDelegate` (delegate `Shoot`) _output_get true true :!label _label))
  (set `self.AttackTimerHandle` _returnvalue))

(event `self.RemoveAttackSpeedMultiplier`
  (set `self.CurrentAttackSpeed` (`self.DefaultAttackSpeed`))
  (goto _label))

(fn `AutoShoot`)

(fn `Play Footstep Sfx`
  (bind _sound_index (`self.Sound Index`))
  (`GameplayStatics.PlaySound2D` (`|GetArrayItem` (`self.Footstep Sfx`) (`self.Sound Index`)) 1.0 (`KismetMathLibrary.RandomFloatInRange` 0.9 1.1) 0.0 null null)
  (`/Engine/EditorBlueprintResources/StandardMacros.IncrementInt` _sound_index
    (:`  `
      (if (>= _sound_index (`KismetArrayLibrary.Array_Length` (`self.Footstep Sfx`)))
        (set `self.Sound Index` 0)))))

(fn `UserConstructionScript`)