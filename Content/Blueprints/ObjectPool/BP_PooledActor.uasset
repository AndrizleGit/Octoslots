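; BP_PooledActor is an actor built for object pooling that starts each play session inactive.
; SetInUse stores the in-use flag and toggles collision, visibility and tick to match it.
; Each call clears the time-to-live timer, and activation restarts it so ReturnToPool deactivates the actor when it expires instead of destroying it.
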(event `self.ReceiveBeginPlay`
  (`self.SetInUse` false))

(event `SetInUse`
  (params (`In Use` :type Boolean))
  (set `self.InUse` `In Use`)
  (`self.SetActorEnableCollision` `In Use`)
  (`self.SetActorHiddenInGame` (not `In Use`))
  (`self.SetActorTickEnabled` `In Use`)
  (`KismetSystemLibrary.K2_ClearAndInvalidateTimerHandle` (`self.TimeToLiveTimer`))
  (if `In Use`
    (bind _returnvalue (`KismetSystemLibrary.K2_SetTimerDelegate` (delegate `ReturnToPool`) (`self.TimeToLive`)))
    (set `self.TimeToLiveTimer` _returnvalue)))

(event `ReturnToPool`
  (`self.SetInUse` false))

(fn `UserConstructionScript`)