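; Actor component that provides an object pool, reusing pre-spawned actors of a configurable class.
; On BeginPlay it spawns a batch sized by PoolSize, stores them in ObjectPool and marks each as not in use.
; SpawnFromPool linearly searches for the first free actor, teleports it to the requested transform and marks it in use.
; When none is available it only prints a failure message, without growing the pool.
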(event `self.ReceiveBeginPlay`
  (`self.InitPool`))

(event `InitPool`
  (for _ (range (+ (`self.PoolSize`) 1))
    (bind _returnvalue (`|SpawnActorFromClass` (`self.PoolActorClass`) (`KismetMathLibrary.MakeTransform` (0.0 0.0 0.0)) "Undefined" "MultiplyWithRoot" null 3.0 null))
    (`KismetArrayLibrary.Array_AddUnique` (`self.ObjectPool`) _returnvalue)
    (`/Game/Blueprints/ObjectPool/BP_PooledActor.SetInUse` _returnvalue false)))

(fn `FindFirstAvailableActor`
  (returns (`Pooled Actor` :type "/Game/Blueprints/ObjectPool/BP_PooledActor Object Reference"))
  (for _array_element (`self.ObjectPool`)
    (if (not (`/Game/Blueprints/ObjectPool/BP_PooledActor.InUse` _array_element))
      (return _array_element))))

(fn `SpawnFromPool`
  (params (SpawnTransform :type "Transform Structure"))
  (returns (PooledActor :type "/Game/Blueprints/ObjectPool/BP_PooledActor Object Reference"))
  (bind _pooled_actor (`self.FindFirstAvailableActor`))
  (`/Engine/EditorBlueprintResources/StandardMacros.IsValid` _pooled_actor
    (:`Is Valid`
      (`Actor.K2_SetActorTransform` _pooled_actor SpawnTransform false true)
      (`/Game/Blueprints/ObjectPool/BP_PooledActor.SetInUse` _pooled_actor true)
      (return _pooled_actor))
    (:`Is Not Valid`
      (`KismetSystemLibrary.PrintString` "Failed to Spawn Actor From Pool"))))