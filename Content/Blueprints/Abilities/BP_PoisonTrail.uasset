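; BP_PoisonTrail is a trail hazard that poisons enemy characters entering its box collision.
; On overlap it applies GE_Debuff_PoisonTrail through the player's Ability System Component, cached at BeginPlay.
; Gameplay tag checks skip enemies that already carry either the PoisonTrail or PlayerPoison debuff.
; The SetinUse override calls its parent and adds no behavior of its own.
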(event `self.ReceiveBeginPlay`
  (set `self.AbilitySystemRef` (`AbilitySystemBlueprintLibrary.GetAbilitySystemComponent` (`GameplayStatics.GetPlayerPawn` 0))))

(event `self.SetInUse`
  (params (`In Use` :type Boolean))
  (`parent.SetInUse` `In Use`)
  (if `In Use`
    _))

(event `self.Box.OnComponentBeginOverlap`
  (params (OverlappedComponent :type "PrimitiveComponent Object Reference") (OtherActor :type "Actor Object Reference") (OtherComp :type "PrimitiveComponent Object Reference") (OtherBodyIndex :type Integer) (bFromSweep :type Boolean) (SweepResult :type "HitResult Structure (by ref)"))
  (bind _returnvalue (`AbilitySystemBlueprintLibrary.GetAbilitySystemComponent` OtherActor))
  (if (`KismetMathLibrary.ClassIsChildOf` (`GameplayStatics.GetObjectClass` OtherActor) "/Game/Blueprints/Enemies/BaseEnemy/BP_BaseEnemyCharacter.BP_BaseEnemyCharacter_C")
    (if (`GameplayTagAssetInterface.HasMatchingGameplayTag` _returnvalue (struct :`TagName` "Debuffs.PoisonTrail"))
      _
      (elif (not (`GameplayTagAssetInterface.HasMatchingGameplayTag` _returnvalue (struct :`TagName` "Debuffs.PlayerPoison")))
        (`AbilitySystemComponent.BP_ApplyGameplayEffectToTarget` :`self` (`self.AbilitySystemRef`) :`GameplayEffectClass` "/Game/GameplayAbilitySystem/Effects/Debuffs/GE_Debuff_PoisonTrail.GE_Debuff_PoisonTrail_C" :`Target` _returnvalue)))))

(fn `UserConstructionScript`)