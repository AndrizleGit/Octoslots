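; Treasure pickup that the octopus player digs up, with a shovel monkey animation.
; Overlapping its sphere starts a looping timer that builds progress toward the TreasureMap's DiggingTime.
; Leaving starts a slower decay timer without clearing the dig timer, and re-entry doesn't clear decay.
; Completion adds a cannon fragment, applies the GE_TreasureReward gameplay effect, destroys the treasure and notifies the player.
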(event `self.ReceiveBeginPlay`
  (bind _returnvalue (`GameplayStatics.GetActorOfClass` "/Game/Blueprints/BP_OctopusCharacter.BP_OctopusCharacter_C"))
  (bind _output_get (set `self.Player Ref` _returnvalue))
  (set `self.TreasureMapRef` (`/Game/Blueprints/BP_OctopusCharacter.TreasureMap` _output_get)))

(event `self.Sphere.OnComponentBeginOverlap`
  (params (OverlappedComponent :type "PrimitiveComponent Object Reference") (OtherActor :type "Actor Object Reference") (OtherComp :type "PrimitiveComponent Object Reference") (OtherBodyIndex :type Integer) (bFromSweep :type Boolean) (SweepResult :type "HitResult Structure (by ref)"))
  (cast `/Game/Blueprints/BP_OctopusCharacter` OtherActor)
  (`KismetSystemLibrary.PrintString` (`KismetStringLibrary.Conv_DoubleToString` (`self.Digging Progress`)))
  (bind _returnvalue (`KismetSystemLibrary.K2_SetTimerDelegate` (delegate `DigTreasure`) 0.5 true))
  (set `self.Digging TimeHandle Ref` _returnvalue))

(event `DigTreasure`
  (bind _player_ref (`self.Player Ref`))
  (bind _shovelmonke (`self.ShovelMonke`))
  (bind _treasuremapref (`self.TreasureMapRef`))
  (`SkeletalMeshComponent.PlayAnimation` _shovelmonke "/Game/Characters/ShovelMonkey/A_ShovelMonke_Transition_001_Anim.A_ShovelMonke_Transition_001_Anim" false)
  (`SkeletalMeshComponent.PlayAnimation` _shovelmonke "/Game/Characters/ShovelMonkey/A_ShovelMonke_Dig_001_Anim.A_ShovelMonke_Dig_001_Anim" false)
  (bind _output_get (set `self.Digging Progress` (+ (`self.Digging Progress`) 0.5)))
  (if (>= _output_get (`TreasureMapComponent.DiggingTime` _treasuremapref))
    (`TreasureMapComponent.AddCannonFragment` _treasuremapref)
    (`KismetSystemLibrary.K2_ClearAndInvalidateTimerHandle` (`self.Digging TimeHandle Ref`))
    (`AbilitySystemComponent.BP_ApplyGameplayEffectToSelf` :`self` (`AbilitySystemBlueprintLibrary.GetAbilitySystemComponent` _player_ref) :`GameplayEffectClass` "/Game/GameplayAbilitySystem/Effects/GE_TreasureReward.GE_TreasureReward_C")
    (`KismetSystemLibrary.PrintString` "Reward Granted")
    (`self.K2_DestroyActor`)
    (`/Game/Blueprints/BP_OctopusCharacter.Treasure Received` _player_ref)))

(event `self.Sphere.OnComponentEndOverlap`
  (params (OverlappedComponent :type "PrimitiveComponent Object Reference") (OtherActor :type "Actor Object Reference") (OtherComp :type "PrimitiveComponent Object Reference") (OtherBodyIndex :type Integer))
  (cast `/Game/Blueprints/BP_OctopusCharacter` OtherActor)
  (`KismetSystemLibrary.PrintString` (`KismetStringLibrary.Conv_DoubleToString` (`self.Digging Progress`)))
  (bind _returnvalue (`KismetSystemLibrary.K2_SetTimerDelegate` (delegate `NotDigging`) 0.5 true))
  (set `self.Not Digging TimeHandle Ref` _returnvalue))

(event `NotDigging`
  (bind _output_get (set `self.Digging Progress` (- (`self.Digging Progress`) 0.25)))
  (if (<= _output_get 0.0)
    (`KismetSystemLibrary.K2_ClearAndInvalidateTimerHandle` (`self.Not Digging TimeHandle Ref`))
    (`KismetSystemLibrary.PrintString` "Dig at 0 %")))

(fn `UserConstructionScript`)