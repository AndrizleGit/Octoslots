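; Treasure map pickup that starts a treasure spawn for the octopus character who collects it.
; On BeginPlay it picks a random mesh from its list and applies paper and handle materials.
; On pickup it asks the character's TreasureMap to spawn treasure in a zone, but only if no valid BP_Treasure is already in the world.
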(event `self.ReceiveBeginPlay`
  (bind _cube (`self.Cube`))
  (`StaticMeshComponent.SetStaticMesh` _cube (`KismetArrayLibrary.Array_Random` (`self.Mesh`)))
  (`PrimitiveComponent.SetMaterial` _cube 0 "/Game/Blueprints/Pickups/Treasure/MS_Paper.MS_Paper")
  (`PrimitiveComponent.SetMaterial` _cube 1 "/Game/Blueprints/Pickups/Treasure/MS_Handle.MS_Handle"))

(event `self.OnPickedUp`
  (params (PickedUpBy :type "Actor Object Reference"))
  (bind _returnvalue (`GameplayStatics.GetActorOfClass` "/Game/Blueprints/Pickups/Treasure/BP_Treasure.BP_Treasure_C"))
  (if (not (`KismetSystemLibrary.IsValid` _returnvalue))
    (bind _asbp_octopus_character (cast `/Game/Blueprints/BP_OctopusCharacter` PickedUpBy))
    (`TreasureMapComponent.SpawnTreasureInZone` (`/Game/Blueprints/BP_OctopusCharacter.TreasureMap` _asbp_octopus_character))))

(fn `UserConstructionScript`)