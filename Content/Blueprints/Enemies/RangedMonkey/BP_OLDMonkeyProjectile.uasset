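; BP_OLDMonkeyProjectile is a reusable projectile for the ranged monkey enemy that damages what it overlaps.
; It extends the parent's SetInUse, launching ProjectileMovement along its forward vector at ProjectileSpeed when activated and zeroing velocity when released.
; A sphere overlap applies ProjectileDamage to the other actor, then releases the projectile through SetInUse rather than destroying it.
; BeginPlay sets TimeToLive, which this graph does not otherwise use.
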(event `self.ReceiveBeginPlay`
  (set `self.TimeToLive` 5.0))

(event `self.SetInUse`
  (params (`In Use` :type Boolean))
  (`parent.SetInUse` `In Use`)
  (if `In Use`
    (set `MovementComponent.Velocity` (* (`self.GetActorForwardVector`) (`self.Projectile Speed`)) (`self.ProjectileMovement`))
    (else
      (set `MovementComponent.Velocity` (0.0 0.0 0.0) (`self.ProjectileMovement`)))))

(event `self.Sphere1.OnComponentBeginOverlap`
  (params (OverlappedComponent :type "PrimitiveComponent Object Reference") (OtherActor :type "Actor Object Reference") (OtherComp :type "PrimitiveComponent Object Reference") (OtherBodyIndex :type Integer) (bFromSweep :type Boolean) (SweepResult :type "HitResult Structure (by ref)"))
  (`GameplayStatics.ApplyDamage` OtherActor (`self.ProjectileDamage`))
  (`self.SetInUse` false))

(fn `UserConstructionScript`)