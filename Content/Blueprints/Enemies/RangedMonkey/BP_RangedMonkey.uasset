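; BP_RangedMonkey is a ranged monkey enemy that fires projectiles drawn from an object pool.
; On BeginPlay it links itself to its health bar widget and caches the level's BP_MonkeyProjectilePool actor.
; ShootProjectile spawns a pooled BP_MonkeyProjectile at the monkey's location and rotation, then sets its damage from the attack damage value in the GAS BasicAttributeSet.
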(event `self.ReceiveBeginPlay`
  (`parent.ReceiveBeginPlay`)
  (bind _aswbp_enemy_health_bar (cast `/Game/UI/Widgets/WBP_EnemyHealthBar` (`WidgetComponent.GetUserWidgetObject` (`self.EnemyHealthBar`))))
  (set `/Game/UI/Widgets/WBP_EnemyHealthBar.EnemyCharacter` self _aswbp_enemy_health_bar)
  (bind _returnvalue (`GameplayStatics.GetActorOfClass` "/Game/Blueprints/Enemies/RangedMonkey/BP_MonkeyProjectilePool.BP_MonkeyProjectilePool_C"))
  (set `self.Projectile Pool Ref` _returnvalue))

(fn `ShootProjectile`
  (bind (_returnvalue_location _returnvalue_rotation) (`KismetMathLibrary.BreakTransform` (`self.GetTransform`)))
  (bind _returnvalue (`AbilitySystemComponent.GetAttributeSet` (`self.AbilitySystemComponent`) "/Script/OctoPirate.BasicAttributeSet"))
  (bind _output_get (set `self.Projectile Pool Ref` (`self.Projectile Pool Ref`)))
  (bind _pooledactor (`/Game/Blueprints/ObjectPool/AC_ObjectPool.SpawnFromPool` (`/Game/Blueprints/Enemies/RangedMonkey/BP_MonkeyProjectilePool.AC_ObjectPool` _output_get) (`KismetMathLibrary.MakeTransform` _returnvalue_location _returnvalue_rotation)))
  (bind _asbp_monkey_projectile (cast `/Game/Blueprints/Enemies/RangedMonkey/BP_MonkeyProjectile` _pooledactor))
  (set `/Game/Blueprints/Enemies/RangedMonkey/BP_MonkeyProjectile.ProjectileDamage` (`BasicAttributeSet.GetAttackDamageValue` _returnvalue) _asbp_monkey_projectile))

(fn `UserConstructionScript`)