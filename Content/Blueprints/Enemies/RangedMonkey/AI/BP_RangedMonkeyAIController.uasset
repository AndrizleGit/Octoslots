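; AI controller for the ranged monkey enemy that starts its behavior tree on possession.
; After casting the pawn to BP_RangedMonkey, it seeds the blackboard with the first player pawn as the target.
; It also copies the monkey's range and fire rate into blackboard keys so the tree uses per-enemy stats.
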(event `self.ReceivePossess`
  (params (PossessedPawn :type "Pawn Object Reference"))
  (`self.RunBehaviorTree` "/Game/Blueprints/Enemies/RangedMonkey/AI/BT_RangedMonkey.BT_RangedMonkey")
  (bind _asbp_ranged_monkey (cast `/Game/Blueprints/Enemies/RangedMonkey/BP_RangedMonkey` PossessedPawn))
  (`BlackboardComponent.SetValueAsObject` (`self.Blackboard`) "TargetPlayer" (`GameplayStatics.GetPlayerPawn` 0))
  (`BlackboardComponent.SetValueAsFloat` (`self.Blackboard`) "Range" (`/Game/Blueprints/Enemies/RangedMonkey/BP_RangedMonkey.Range` _asbp_ranged_monkey))
  (`BlackboardComponent.SetValueAsFloat` (`self.Blackboard`) "Firerate" (`/Game/Blueprints/Enemies/RangedMonkey/BP_RangedMonkey.Firerate` _asbp_ranged_monkey)))

(fn `UserConstructionScript`)