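; BP_Blockade is a destructible blockade that takes a set number of cannon shots to clear.
; On BeginPlay it binds to the cannon shot event and caches BP_OctopusCharacter and its own blockade level.
; Each shot decrements ShootRequirement and calls Explode.
; When the requirement reaches zero, it destroys itself and passes its level to the octopus character's TreasureMap via SetTreasureLevel.
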(event `Blockade Exploding`
  (bind _output_get (set `self.ShootRequirement` (- (`self.ShootRequirement`) 1.0)))
  (`self.Explode`)
  (if (<= _output_get 0.0)
    (`self.K2_DestroyActor`)
    (`TreasureMapComponent.SetTreasureLevel` (`/Game/Blueprints/BP_OctopusCharacter.TreasureMap` (stale `self.ReceiveBeginPlay` _returnvalue)) (stale `self.ReceiveBeginPlay` _output_get))))

(event `self.ReceiveBeginPlay`
  (add `self.Cannon Shot` (delegate `Blockade Exploding`))
  (bind _returnvalue (`GameplayStatics.GetActorOfClass` "/Game/Blueprints/BP_OctopusCharacter.BP_OctopusCharacter_C"))
  (bind _returnvalue_2 (`self.GetBlockadeLevel`))
  (bind _output_get (set `self.BlockadeLevelRef` _returnvalue_2)))

(fn `UserConstructionScript`)