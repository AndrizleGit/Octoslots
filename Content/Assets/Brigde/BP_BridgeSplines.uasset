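; Bridge actor that procedurally builds a plank-and-rope bridge along a spline in the construction script.
; It divides the spline by plank mesh length, adding spline mesh segments for randomly picked planks and two offset, raised ropes with length-clamped tangents.
; AddPole places random, yaw-aligned, sunken pole meshes on both sides at each end, called inside the segment loop so they repeat every iteration.
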(fn `AddPole`
  (params (Distance :type "Float (double-precision)") (Side :type "Float (double-precision)" :default 1.0))
  (bind _spline (`self.Spline`))
  (bind _returnvalue (`AddComponent|NODE_AddStaticMeshComponent-1`))
  (`PrimitiveComponent.SetCollisionEnabled` _returnvalue "QueryAndPhysics")
  (`StaticMeshComponent.SetStaticMesh` _returnvalue (`KismetArrayLibrary.Array_Random` (`self.PoleMeshes`)))
  (`SceneComponent.K2_SetWorldLocationAndRotation` _returnvalue (+ (+ (`SplineComponent.GetLocationAtDistanceAlongSpline` _spline Distance "World") (* (`SplineComponent.GetRightVectorAtDistanceAlongSpline` _spline Distance "World") (* (`self.HalfRopeDistance`) Side))) (`KismetMathLibrary.MakeVector` 0.0 0.0 (* (`self.SinkAmount`) -1.0))) (`KismetMathLibrary.MakeRotator` 0.0 0.0 (.yaw (`SplineComponent.GetRotationAtDistanceAlongSpline` _spline Distance "World"))) false false))

(fn `AddSegment`
  (params (Mesh :type "StaticMesh Object Reference") (StartPosition :type "Vector Structure") (StartTangent :type "Vector Structure") (EndPosition :type "Vector Structure") (EndTangent :type "Vector Structure") (Scale :type "Vector2D Structure"))
  (bind _returnvalue (`AddComponent|NODE_AddSplineMeshComponent-1`))
  (`PrimitiveComponent.SetCollisionEnabled` _returnvalue "QueryAndPhysics")
  (`SplineMeshComponent.SetForwardAxis` _returnvalue "X" true)
  (`StaticMeshComponent.SetStaticMesh` _returnvalue Mesh)
  (`SplineMeshComponent.SetStartAndEnd` _returnvalue StartPosition StartTangent EndPosition EndTangent true)
  (`SplineMeshComponent.SetStartScale` _returnvalue Scale true)
  (`SplineMeshComponent.SetEndScale` _returnvalue Scale true))

(fn `UserConstructionScript`
  (bind _spline (`self.Spline`))
  (bind _spline_2 (`self.Spline`))
  (bind _spline_3 (`self.Spline`))
  (bind (_returnvalue_min _returnvalue_max) (break `Box` (`StaticMesh.GetBoundingBox` (`self.PlankMesh`))))
  (bind _returnvalue (`KismetMathLibrary.MakeVector` 0.0 0.0 (`self.RopeHeight`)))
  (bind _returnvalue_x (`KismetMathLibrary.BreakVector` (+ (`KismetMathLibrary.Vector_GetAbs` _returnvalue_min) (`KismetMathLibrary.Vector_GetAbs` _returnvalue_max))))
  (set `self.HalfRopeDistance` (* (`self.RopeDistance`) 0.5))
  (bind _output_get (set `self.XLength` _returnvalue_x))
  (for _index (range (+ (`KismetMathLibrary.FTrunc` (/ (`SplineComponent.GetSplineLength` (`self.Spline`)) _output_get)) 1))
    (bind _returnvalue_2 (* _index (`self.XLength`)))
    (bind _returnvalue_3 (`SplineComponent.GetLocationAtDistanceAlongSpline` _spline_3 _returnvalue_2 "Local"))
    (bind _returnvalue_4 (`KismetMathLibrary.ClampVectorSize` (`SplineComponent.GetTangentAtDistanceAlongSpline` _spline_3 _returnvalue_2 "Local") 0.0 (`self.XLength`)))
    (bind _returnvalue_5 (* (+ _index 1) (`self.XLength`)))
    (bind _returnvalue_6 (`SplineComponent.GetLocationAtDistanceAlongSpline` _spline_2 _returnvalue_5 "Local"))
    (bind _returnvalue_7 (`KismetMathLibrary.ClampVectorSize` (`SplineComponent.GetTangentAtDistanceAlongSpline` _spline_2 _returnvalue_5 "Local") 0.0 (`self.XLength`)))
    ; Planks
    (`self.AddSegment` (`KismetArrayLibrary.Array_Random` (`self.PlankMeshes`)) _returnvalue_3 _returnvalue_4 _returnvalue_6 _returnvalue_7 (1.0 1.0))
    (bind _returnvalue_8 (* (`SplineComponent.GetRightVectorAtDistanceAlongSpline` _spline _returnvalue_2 "Local") (`self.HalfRopeDistance`)))
    (bind _returnvalue_9 (* (`SplineComponent.GetRightVectorAtDistanceAlongSpline` _spline _returnvalue_5 "Local") (`self.HalfRopeDistance`)))
    ; Left Rope
    (`self.AddSegment` (`self.RopeMesh`) (+ (- _returnvalue_3 _returnvalue_8) _returnvalue) _returnvalue_4 (+ (- _returnvalue_6 _returnvalue_9) _returnvalue) _returnvalue_7 (`KismetMathLibrary.Conv_DoubleToVector2D` (`self.RopeRadius`)))
    ; Right Rope
    (`self.AddSegment` (`self.RopeMesh`) (+ (+ _returnvalue_3 _returnvalue_8) _returnvalue) _returnvalue_4 (+ (+ _returnvalue_6 _returnvalue_9) _returnvalue) _returnvalue_7 (`KismetMathLibrary.Conv_DoubleToVector2D` (`self.RopeRadius`)))
    (`self.AddPole` 0.0)
    (`self.AddPole` (`SplineComponent.GetSplineLength` (`self.Spline`)))
    (`self.AddPole` 0.0 -1.0)
    (`self.AddPole` (`SplineComponent.GetSplineLength` (`self.Spline`)) -1.0)))